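; AI director component that throttles enemy attacks on its owner, apparently the player, in free-flow style combat.
; Registered enemies start a randomized-interval looping timer, cleared when the list empties.
; Each check skips while AC_FFCC holds a counter enemy or a finisher runs.
; Otherwise, if no living enemy is attacking, it flags a random one through AC_EnemyComp, though each Random read may return a different enemy.
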(event EventBeginPlay)

(event EventTick
  (params (DeltaSeconds :type Float%20%28single-precision%29))
  (Development|PrintString (Utilities|String|ToString(Integer) (Utilities|Array|Length (Variables|Default|GetEnemy%20Ref))) true true "(R=1.000000,G=0.426703,B=0.000000,A=1.000000)" 0.0))

(fn AddEnemy
  (params (EnemyRef :type Actor%20Object%20Reference))
  (Utilities|Array|AddUnique (Variables|Default|GetEnemy%20Ref) EnemyRef)
  (if (and (> (Utilities|Array|Length (Variables|Default|GetEnemy%20Ref)) 0) (not (Utilities|Time|IsTimerActivebyHandle (Variables|Default|GetCheck%20Attack%20Player))))
    (bind _returnvalue (Utilities|Time|SetTimerbyFunctionName 0 "Check If Player Under Attack" (Math|Random|RandomFloatinRange 5.0 8.0) true))
    (Variables|Default|SetCheck%20Attack%20Player _returnvalue)))

(fn RemoveEnemy
  (params (EnemyRef :type Actor%20Object%20Reference))
  (Utilities|Array|RemoveItem (Variables|Default|GetEnemy%20Ref) EnemyRef)
  (if (<= (Utilities|Array|Length (Variables|Default|GetEnemy%20Ref)) 0)
    (Utilities|Time|ClearandInvalidateTimerbyHandle (Variables|Default|GetCheck%20Attack%20Player))))

(fn CheckifPlayerUnderAttack
  (bind _returnvalue (Components|GetOwner))
  (bind _enemy_ref (Variables|Default|GetEnemy%20Ref))
  (bind _outitem (Utilities|Array|Random _enemy_ref))
  (bind _returnvalue_2 (Actor|GetComponentbyClass _returnvalue "/Game/NoahsFolder/FFCS/AC_FFCC.AC_FFCC_C"))
  (bind _returnvalue_3 (Actor|GetComponentbyClass _outitem "/Game/NoahsFolder/FFCS/AC_EnemyComp.AC_EnemyComp_C"))
  (Utilities|IsValid _returnvalue_2
    (:Is%20Valid
      (Utilities|IsValid (Class|ACFFCCBase|GetCounterEnemy _returnvalue_2)
        (:Is%20Valid
          (Development|PrintString "Last Enemy Not Cleared" true true "(R=1.000000,G=0.793096,B=0.000000,A=1.000000)"))
        (:Is%20Not%20Valid
          (if (GameplayTags|MatchesAnyTags (Class|ACFFCCBase|GetTag _returnvalue_2) (GameplayTags|MakeLiteralGameplayTagContainer "(GameplayTags=((TagName=\"PlayerStates.FinisherInProgress\"),(TagName=\"PlayerStates.Finisher\")))"))
            (Development|PrintString "Finisher Active" true true "(R=1.000000,G=0.000000,B=0.457612,A=1.000000)" 4.0)
            (else
              (LocalVariables|SetChoose%20AI%20To%20Attack true :!label _label)
              (for _array_element (Variables|Default|GetEnemy%20Ref)
                (Utilities|IsValid (Actor|GetComponentbyClass _array_element "/Game/NoahsFolder/FFCS/AC_EnemyComp.AC_EnemyComp_C")
                  (:Is%20Valid
                    (if (and (Default|GetAttackPlayer (Actor|GetComponentbyClass _array_element "/Game/NoahsFolder/FFCS/AC_EnemyComp.AC_EnemyComp_C")) (not (Variables|/Script/Lighting2.AC_EnemyComp_Base|GetbDead (Actor|GetComponentbyClass _array_element "/Game/NoahsFolder/FFCS/AC_EnemyComp.AC_EnemyComp_C"))))
                      (LocalVariables|SetChoose%20AI%20To%20Attack false)))))
              (if (LocalVariables|GetChoose%20AI%20To%20Attack)
                (Utilities|IsValid _outitem
                  (:Is%20Valid
                    (Utilities|IsValid _returnvalue_3
                      (:Is%20Valid
                        (if (not (Variables|/Script/Lighting2.AC_EnemyComp_Base|GetbDead _returnvalue_3))
                          (Class|ACEnemyCompBase|SetAttackPlayer _returnvalue_3 true))))))))))))
    (:Is%20Not%20Valid
      (goto _label))))