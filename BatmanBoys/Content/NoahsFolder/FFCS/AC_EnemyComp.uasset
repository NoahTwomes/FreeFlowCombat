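; Enemy-side combat component for Goon characters, pairing with the player's AC_FFCC in free-flow-style melee with hits, counters and finishers.
; Reaction montages end by releasing the attack flag, randomizing the blackboard AI state and restarting logic on a timer.
; Attacking registers the owner as the player's counter enemy, cleared again after counters or matching hits.
; It also tracks health and death, computes hit direction, and toggles AI logic with movement avoidance.
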(event Custom|PlayHitMontage
  (params (HitDirection :type EAttackHitDirection%20Enum :default "Fwd"))
  ;[1 1 1] Enemy Hit Montage Logic
  (Animation|Montage|PlayMontage (Variables|/Script/Engine.Character|GetMesh (Variables|Default|GetAs%20Goon)) (Utilities|Select :Index HitDirection :Fwd "/Game/ARPG_Unarmed_Anim_UE_Hit6_Montage.ARPG_Unarmed_Anim_UE_Hit6_Montage" :Bwd "/Game/ARPG_Unarmed_Anim_UE_Hit11_Montage.ARPG_Unarmed_Anim_UE_Hit11_Montage" :Lt "/Game/ARPG_Unarmed_Anim_UE_Hit1_Montage.ARPG_Unarmed_Anim_UE_Hit1_Montage" :Rt "/Game/ARPG_Unarmed_Anim_UE_Hit2_Montage.ARPG_Unarmed_Anim_UE_Hit2_Montage")
    (:then
      (bind _returnvalue (CallFunction|CheckCurrentandCounterEnemy))
      (if _returnvalue
        (CallFunction|SetAttackPlayer false)
        (CallFunction|ResetCounterEnemyinPlayer)
        (CallFunction|SetAIStatetoRandom)
        (elif (CallFunction|GetAttackPlayer)
          (CallFunction|SetAttackPlayer false)
          (CallFunction|SetAIStatetoRandom))))
    (:OnCompleted
      (bind _returnvalue_2 (Utilities|Time|SetTimerbyFunctionName 0 "StartLogic" 1.0 :!label _label))
      (Variables|Default|SetStartLogicTH _returnvalue_2))
    (:OnBlendOut
      (goto _label))
    (:OnInterrupted
      (goto _label))))

(event Custom|PlayCounterDamage
  (params (MontageToPlay :type Anim%20Montage%20Object%20Reference))
  ;[1 1 1] Enemy Counter Montage Logic
  (Animation|Montage|PlayMontage (Variables|/Script/Engine.Character|GetMesh (Variables|Default|GetAs%20Goon)) MontageToPlay
    (:OnCompleted
      _)
    (:OnBlendOut
      _)
    (:OnInterrupted
      _))
  (bind _returnvalue (Utilities|Time|SetTimerbyFunctionName 0 "StartLogic" 1.0))
  (Variables|Default|SetStartLogicTH _returnvalue)
  (CallFunction|SetAttackPlayer false)
  (CallFunction|ResetCounterEnemyinPlayer)
  (CallFunction|SetAIStatetoRandom))

(event Custom|PlayFinisher
  (params (MontageToPlay :type Anim%20Montage%20Object%20Reference))
  ;[1 1 1] Enemy Finisher Montage Logic
  (Animation|Montage|PlayMontage (Variables|/Script/Engine.Character|GetMesh (Variables|Default|GetAs%20Goon)) MontageToPlay
    (:OnCompleted
      _)
    (:OnBlendOut
      _)
    (:OnInterrupted
      _))
  (bind _returnvalue (Utilities|Time|SetTimerbyFunctionName 0 "StartLogic" 3.0))
  (Variables|Default|SetStartLogicTH _returnvalue)
  (bind _returnvalue_2 (CallFunction|CheckCurrentandCounterEnemy))
  (if _returnvalue_2
    (CallFunction|SetAttackPlayer false)
    (CallFunction|ResetCounterEnemyinPlayer)
    (CallFunction|SetAIStatetoRandom)
    (elif (CallFunction|GetAttackPlayer)
      (CallFunction|SetAttackPlayer false)
      (CallFunction|SetAIStatetoRandom))))

(event EventBeginPlay
  (bind _asgoon (Utilities|Casting|CastToGoon (Components|GetOwner)))
  (Variables|Default|SetAs%20Goon _asgoon))

(event EventSetCurrentHealth
  (params (Damage :type Float%20%28single-precision%29%20%28by%20ref%29))
  ;[1 1 1] Set Current Health
  (bind _output_get (Variables|Default|SetCurrentHealth (Math|Float|Clamp(Float) (- (CallFunction|GetCurrentHealth) Damage) 0.0 (CallFunction|GetMaxHealth))))
  (Development|PrintString (Utilities|String|ToString(Float) _output_get) true true "(R=0.000000,G=1.000000,B=0.277591,A=1.000000)" 4.0))

(event EventSetEnemyDead
  (params (ActorDead :type Boolean))
  (Variables|Default|SetbDead ActorDead))

(fn GetHitDirection
  (params (Instigator :type Actor%20Object%20Reference))
  (bind _returnvalue (Components|GetOwner))
  (bind _returnvalue_2 (Transformation|GetActorLocation Instigator))
  (bind _returnvalue_3 (Transformation|GetActorLocation _returnvalue))
  (bind _returnvalue_4 (Transformation|GetActorRotation _returnvalue))
  (bind _returnvalue_5 (Math|Rotator|FindLookatRotation _returnvalue_3 _returnvalue_2))
  (bind _returnvalue_6 (Math|Rotator|Delta(Rotator) _returnvalue_5 _returnvalue_4))
  (if (Math|Float|InRange(Float) (.yaw _returnvalue_6) -45.0 45.0)
    (Development|PrintString "forward")
    (return "Fwd")
    (elif (Math|Float|InRange(Float) (.yaw _returnvalue_6) 45.0 135.0)
      (Development|PrintString "right")
      (return "Rt")
      (elif (or (Math|Float|InRange(Float) (.yaw _returnvalue_6) 135.0 1.8e+02) (Math|Float|InRange(Float) (.yaw _returnvalue_6) -179.99 -135.0))
        (Development|PrintString "back")
        (return "Bwd")
        (else
          (Development|PrintString "left")
          (return "Lt"))))))

(fn StopEnemyLogic
  (params (Stop :type Boolean))
  (bind _returnvalue (Components|GetOwner))
  (bind _returnvalue_2 (AI|GetAIController _returnvalue))
  (if Stop
    (Utilities|Time|ClearandInvalidateTimerbyHandle (Variables|Default|GetStartLogicTH))
    (Utilities|IsValid (AI|GetAIController (Components|GetOwner))
      (:Is%20Valid
        (Utilities|IsValid _returnvalue_2
          (:Is%20Valid
            (AI|Logic|StopLogic (Variables|/Script/AIModule.AIController|GetBrainComponent _returnvalue_2) "Being Attacked")
            (CallFunction|StopMovementAvoidance true)))))
    (else
      (Utilities|IsValid (AI|GetAIController (Components|GetOwner))
        (:Is%20Valid
          (Utilities|IsValid _returnvalue_2
            (:Is%20Valid
              (AI|Logic|StartLogic (Variables|/Script/AIModule.AIController|GetBrainComponent (AI|GetAIController (Components|GetOwner))))
              (CallFunction|StopMovementAvoidance false))))))))

(fn StopMovementAvoidance
  (params (Stop :type Boolean))
  (bind _returnvalue (Components|GetOwner))
  (bind _returnvalue_2 (Actor|GetComponentbyClass _returnvalue "/Script/Engine.CharacterMovementComponent"))
  (Utilities|IsValid _returnvalue_2
    (:Is%20Valid
      (Class|CharacterMovementComponent|SetAvoidanceEnabled _returnvalue_2 (not Stop)))))

(fn StartLogic
  (CallFunction|StopEnemyLogic false))

(fn GetAttackPlayer
  (return (Variables|Default|GetAttacking%20Player)))

(fn GetEnemyTeleportLocation
  (params (Offset :type Float%20%28double-precision%29))
  (bind _returnvalue (Components|GetOwner))
  (bind _returnvalue_2 (Components|GetOwner))
  (bind _returnvalue_3 (Utilities|Name|MakeLiteralName "TargetActor"))
  (bind _returnvalue_4 (AI|GetBlackboard _returnvalue))
  (bind _returnvalue_5 (Transformation|GetActorLocation _returnvalue_2))
  (bind _returnvalue_6 (AI|Components|Blackboard|GetValueasObject _returnvalue_4 _returnvalue_3))
  (bind _ascharacter (Utilities|Casting|CastToCharacter _returnvalue_6))
  (bind _returnvalue_7 (Transformation|GetActorLocation _ascharacter))
  (return (+ (* (Math|Vector|Normalize (- _returnvalue_5 _returnvalue_7)) Offset) _returnvalue_7) (Math|Rotator|FindLookatRotation _returnvalue_5 _returnvalue_7)))

(fn HitDirection
  (params (Instigator :type Actor%20Object%20Reference))
  (bind _returnvalue (|CallParentFunction Instigator))
  (return _returnvalue))

(fn SetAttackPlayer
  (params (AttackPlayer :type Boolean))
  (bind _returnvalue (Components|GetOwner))
  (bind _returnvalue_2 (Components|GetOwner))
  (bind _returnvalue_3 (Utilities|Name|MakeLiteralName "TargetActor"))
  (bind _returnvalue_4 (Components|GetOwner))
  (bind _returnvalue_5 (AI|GetBlackboard _returnvalue))
  (bind _returnvalue_6 (AI|GetBlackboard _returnvalue_4))
  (bind _returnvalue_7 (AI|Components|Blackboard|GetValueasObject _returnvalue_6 _returnvalue_3))
  (bind _ascharacter (Utilities|Casting|CastToCharacter _returnvalue_7))
  (bind _returnvalue_8 (Actor|GetComponentbyClass _ascharacter "/Game/NoahsFolder/FFCS/AC_FFCC.AC_FFCC_C"))
  (bind _output_get (Variables|Default|SetAttacking%20Player AttackPlayer))
  (if _output_get
    (Utilities|IsValid _returnvalue_5
      (:Is%20Valid
        (bind _output_get_2 (LocalVariables|SetAI%20State "Attack"))
        (AI|Components|Blackboard|SetValueasEnum _returnvalue_5 (Utilities|Name|MakeLiteralName "AIStates") _output_get_2)
        (Utilities|IsValid _returnvalue_8
          (:Is%20Valid
            (Class|ACFFCCBase|SetCounterEnemy _returnvalue_8 _returnvalue_2)
            (Development|PrintString (Utilities|GetDisplayName _returnvalue_2) true true "(R=1.000000,G=0.000000,B=0.000000,A=1.000000)" 1e+01))))
      (:Is%20Not%20Valid
        _)))
  (return))

(fn GetAttackPlayer
  (return (Variables|Default|GetAttacking%20Player)))

(fn SetAIStatetoRandom
  (bind _returnvalue (Components|GetOwner))
  (bind _returnvalue_2 (AI|GetBlackboard _returnvalue))
  (Utilities|IsValid _returnvalue_2
    (:Is%20Valid
      (AI|Components|Blackboard|SetValueasEnum _returnvalue_2 (Utilities|Name|MakeLiteralName "AIStates") (.OutItem (Utilities|Array|Random (Utilities|Array|MakeArray "GetBack" "Wait" "LookForWeapons" "Strafe")))))))

(fn ResetCounterEnemyinPlayer
  (bind _returnvalue (Utilities|Name|MakeLiteralName "TargetActor"))
  (bind _returnvalue_2 (Components|GetOwner))
  (bind _returnvalue_3 (AI|GetBlackboard _returnvalue_2))
  (bind _returnvalue_4 (AI|Components|Blackboard|GetValueasObject _returnvalue_3 _returnvalue))
  (Utilities|IsValid _returnvalue_3
    (:Is%20Valid
      (Utilities|IsValid _returnvalue_4
        (:Is%20Valid
          (bind _ascharacter (Utilities|Casting|CastToCharacter _returnvalue_4))
          (Utilities|IsValid (Actor|GetComponentbyClass _ascharacter "/Game/NoahsFolder/FFCS/AC_FFCC.AC_FFCC_C")
            (:Is%20Valid
              (Class|ACFFCCBase|SetCounterEnemy (Actor|GetComponentbyClass _ascharacter "/Game/NoahsFolder/FFCS/AC_FFCC.AC_FFCC_C")))))
        (:Is%20Not%20Valid
          (Development|PrintString "Target Actor Retrive Failed" :!label _label))))
    (:Is%20Not%20Valid
      (goto _label))))

(fn CheckCurrentandCounterEnemy
  (bind _returnvalue (Utilities|Name|MakeLiteralName "TargetActor"))
  (bind _returnvalue_2 (Components|GetOwner))
  (bind _returnvalue_3 (AI|GetBlackboard _returnvalue_2))
  (bind _returnvalue_4 (AI|Components|Blackboard|GetValueasObject _returnvalue_3 _returnvalue))
  (Utilities|IsValid _returnvalue_3
    (:Is%20Valid
      (Utilities|IsValid _returnvalue_4
        (:Is%20Valid
          (bind _ascharacter (Utilities|Casting|CastToCharacter _returnvalue_4))
          (Utilities|IsValid (Actor|GetComponentbyClass _ascharacter "/Game/NoahsFolder/FFCS/AC_FFCC.AC_FFCC_C")
            (:Is%20Valid
              (return (== (Class|ACFFCCBase|GetCurrentEnemy (Actor|GetComponentbyClass _ascharacter "/Game/NoahsFolder/FFCS/AC_FFCC.AC_FFCC_C")) (Class|ACFFCCBase|GetCounterEnemy (Actor|GetComponentbyClass _ascharacter "/Game/NoahsFolder/FFCS/AC_FFCC.AC_FFCC_C")))))
            (:Is%20Not%20Valid
              (return false))))
        (:Is%20Not%20Valid
          (Development|PrintString "Target Actor Retrive Failed"))))))

(fn GetCurrentHealth
  (return (Variables|Default|GetCurrentHealth)))

(fn GetMaxHealth
  (return (Variables|Default|GetMaxHealth)))

(fn GetEnemyDead
  (return (Variables|Default|GetbDead)))