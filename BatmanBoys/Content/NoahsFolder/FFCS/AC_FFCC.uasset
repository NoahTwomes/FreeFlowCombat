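; Player combat component for free-flow melee, tracking current and counter enemies, a gameplay-tag player state, and attack and finisher animation data.
; It plays directional hit reactions, counters and finishers, driving the paired enemy reactions and pausing or resuming enemy logic through AC_EnemyComp.
; A timed combo counter updates the HUD and arms a finisher every sixth count, while hit reactions reset it.
; Helpers pick montages by distance and resolve hit direction from yaw.
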(event EventBeginPlay)

(event EventSetFinisherAnims
  (params (NewFinisherData :type Player%20Finisher%20Data%20Structure%20%28by%20ref%29))
  (Variables|Default|SetFinisherAnims NewFinisherData))

(event EventPlayFinisherMontage
  (bind _returnvalue (CallFunction|GetFinisherAnims))
  (bind (_finishermontage _hitmontage) (Utilities|Struct|BreakPlayerFinisherData _returnvalue))
  ;[1 1 1] Finisher Montage Logic
  (Animation|Montage|PlayMontage (Actor|GetComponentbyClass (Components|GetOwner) "/Script/Engine.SkeletalMeshComponent") _finishermontage
    (:then
      (Default|PlayFinisher (Actor|GetComponentbyClass (CallFunction|GetCurrentEnemy) "/Game/NoahsFolder/FFCS/AC_EnemyComp.AC_EnemyComp_C") _hitmontage))))

(event EventPlayHitMontage
  (params (HitDirection :type EAttackHitDirection%20Enum :default "Fwd"))
  (bind _returnvalue (CallFunction|GetCurrentEnemy))
  (bind _returnvalue_2 (Components|GetOwner))
  (bind _returnvalue_3 (Actor|GetComponentbyClass _returnvalue "/Game/NoahsFolder/FFCS/AC_EnemyComp.AC_EnemyComp_C"))
  (bind _returnvalue_4 (Actor|GetComponentbyClass _returnvalue_2 "/Script/Engine.SkeletalMeshComponent"))
  ;[1 1 1] Hit Montage Logic
  (Utilities|IsValid _returnvalue_4
    (:Is%20Valid
      (Animation|Montage|PlayMontage _returnvalue_4 (Utilities|Select :Index HitDirection :Fwd "/Game/ARPG_Unarmed_Anim_UE_Hit6_Montage.ARPG_Unarmed_Anim_UE_Hit6_Montage" :Bwd "/Game/ARPG_Unarmed_Anim_UE_Hit11_Montage.ARPG_Unarmed_Anim_UE_Hit11_Montage" :Lt "/Game/ARPG_Unarmed_Anim_UE_Hit1_Montage.ARPG_Unarmed_Anim_UE_Hit1_Montage" :Rt "/Game/ARPG_Unarmed_Anim_UE_Hit2_Montage.ARPG_Unarmed_Anim_UE_Hit2_Montage")
        (:then
          (Class|ACFFCCBase|ResetComboCounter)
          (CallFunction|SetTag (GameplayTags|MakeLiteralGameplayTag "(TagName=\"PlayerStates.HitReact\")"))
          (Utilities|IsValid _returnvalue
            (:Is%20Valid
              (Utilities|IsValid _returnvalue_3
                (:Is%20Valid
                  (Default|StopEnemyLogic _returnvalue_3 false))))))
        (:OnCompleted
          (CallFunction|SetTag (GameplayTags|MakeLiteralGameplayTag "(TagName=\"PlayerStates.Idle\")")))))))

(event EventSetCurrentEnemy
  (params (EnemyRef :type Actor%20Object%20Reference))
  (bind _output_get (Variables|Default|SetCurrentEnemy EnemyRef))
  (Utilities|IsValid (Actor|GetComponentbyClass _output_get "/Game/NoahsFolder/FFCS/AC_EnemyComp.AC_EnemyComp_C")
    (:Is%20Valid
      (Default|StopEnemyLogic (Actor|GetComponentbyClass _output_get "/Game/NoahsFolder/FFCS/AC_EnemyComp.AC_EnemyComp_C") true))))

(event EventSetCounterEnemy
  (params (EnemyRef :type Actor%20Object%20Reference))
  (Variables|Default|SetCounter%20Enemy EnemyRef))

(event EventPlayCounterMontage
  (bind _returnvalue (CallFunction|GetCounterEnemy))
  ;[1 1 1] Counter montage logic
  (Animation|Montage|PlayMontage (Actor|GetComponentbyClass (Components|GetOwner) "/Script/Engine.SkeletalMeshComponent") "/Game/Finisher_Animations/Animations/Counter/AM_P_C_001.AM_P_C_001"
    (:then
      (Utilities|IsValid _returnvalue
        (:Is%20Valid
          (Default|PlayCounterDamage (Actor|GetComponentbyClass _returnvalue "/Game/NoahsFolder/FFCS/AC_EnemyComp.AC_EnemyComp_C") "/Game/Finisher_Animations/Animations/Counter/AM_AI_HCD_001.AM_AI_HCD_001")
          (CallFunction|SetTag (GameplayTags|MakeLiteralGameplayTag "(TagName=\"PlayerStates.Idle\")")))))
    (:OnCompleted
      (CallFunction|SetTag (GameplayTags|MakeLiteralGameplayTag "(TagName=\"PlayerStates.Idle\")") :!label _label))
    (:OnBlendOut
      (goto _label))))

(event EventComboCounter
  (bind _hud_ref (Variables|Default|GetHUD%20Ref))
  (bind _ui_player_hud_ref (Variables|/Game/NoahsFolder/HUD/BP_Hud_Main.BP_Hud_Main_C|GetUI%20Player%20HUD%20Ref _hud_ref))
  ;[1 1 1] Set Combo Counter Logic
  (bind _result (Math|Integer|IncrementInt (Variables|Default|GetCounter))
    (:%20%20
      (Default|SetCounterValue _ui_player_hud_ref _result)
      (Default|SetCounterVisibility _ui_player_hud_ref "Visible" 0.1)
      (Utilities|Time|ClearandInvalidateTimerbyHandle (Variables|Default|GetComboCounter_TimerHandle))
      (bind _returnvalue (Utilities|Time|SetTimerbyEvent (EventDispatchers|CreateEvent :!event ResetComboCounter) 3.0))
      (Variables|Default|SetComboCounter_TimerHandle _returnvalue)
      (if (== (Math|Integer|%(Integer) (Variables|Default|GetCounter) 6) 0)
        (CallFunction|SetFinisher true)
        (elif (not (CallFunction|GetFinisher))
          (CallFunction|SetFinisher false))))))

(event EventResetComboCounter
  (bind _hud_ref (Variables|Default|GetHUD%20Ref))
  (bind _ui_player_hud_ref (Variables|/Game/NoahsFolder/HUD/BP_Hud_Main.BP_Hud_Main_C|GetUI%20Player%20HUD%20Ref _hud_ref))
  ;[1 1 1] Reset Combo Counter
  (Variables|Default|SetCounter 0)
  (CallFunction|SetFinisher false)
  (Default|SetCounterValue _ui_player_hud_ref)
  (Default|SetCounterVisibility _ui_player_hud_ref "Hidden" 2.0))

(event EventTick
  (params (DeltaSeconds :type Float%20%28single-precision%29))
  (Development|PrintString (Utilities|String|ToString(Name) (GameplayTags|GetTagName (CallFunction|GetTag))) true true "(R=0.000000,G=0.660000,B=1.000000,A=1.000000)" 0.0))

(event EventSetAttackAnims
  (params (NewAttackData :type Player%20Attack%20Anim%20Data%20Structure%20%28by%20ref%29))
  (Variables|Default|SetAttackAnims NewAttackData))

(fn GetCurrentTag
  (return (Variables|Default|GetPlayer%20State%20Tag)))

(fn GetMontageBasedonDistance
  (bind _returnvalue (Components|GetOwner))
  (bind _returnvalue_2 (CallFunction|GetCurrentEnemy))
  (bind _returnvalue_3 (Transformation|GetActorLocation _returnvalue))
  (bind _returnvalue_4 (Transformation|GetActorLocation _returnvalue_2))
  (bind _returnvalue_5 (Math|Vector|Distance(Vector) _returnvalue_4 _returnvalue_3))
  (if (Math|Float|InRange(Float) _returnvalue_5 0.0 (Utilities|Array|Get(acopy) (Variables|Default|GetDistance)) true false)
    (return (Variables|Default|GetClose%20Combat%20Montage))
    (elif (Math|Float|InRange(Float) _returnvalue_5 (Utilities|Array|Get(acopy) (Variables|Default|GetDistance)) (Utilities|Array|Get(acopy) (Variables|Default|GetDistance) 1))
      (return (Variables|Default|GetMid%20Range%20Combat%20Montage))
      (else
        (return (Variables|Default|GetJump%20Combat%20Montage))))))

(fn HitDirection
  (params (Instigator :type Actor%20Object%20Reference))
  (bind _returnvalue (Components|GetOwner))
  (bind _returnvalue_2 (Transformation|GetActorLocation Instigator))
  (bind _returnvalue_3 (Transformation|GetActorLocation _returnvalue))
  (bind _returnvalue_4 (Transformation|GetActorRotation _returnvalue))
  (bind _returnvalue_5 (Math|Rotator|FindLookatRotation _returnvalue_3 _returnvalue_2))
  (bind _returnvalue_6 (Math|Rotator|Delta(Rotator) _returnvalue_5 _returnvalue_4))
  (if (Math|Float|InRange(Float) (.yaw _returnvalue_6) -45.0 45.0)
    (Development|PrintString "forward")
    (return "Fwd")
    (elif (Math|Float|InRange(Float) (.yaw _returnvalue_6) 45.0 135.0)
      (Development|PrintString "right")
      (return "Rt")
      (elif (or (Math|Float|InRange(Float) (.yaw _returnvalue_6) 135.0 1.8e+02) (Math|Float|InRange(Float) (.yaw _returnvalue_6) -179.99 -135.0))
        (Development|PrintString "back")
        (return "Bwd")
        (else
          (Development|PrintString "left")
          (return "Lt"))))))

(fn GetCurrentEnemy
  (return (Variables|Default|GetCurrentEnemy)))

(fn SetTag
  (params (Tag :type Gameplay%20Tag%20Structure%20%28by%20ref%29))
  (Variables|Default|SetPlayer%20State%20Tag Tag)
  (return))

(fn GetTag
  (return (Variables|Default|GetPlayer%20State%20Tag)))

(fn GetCounterEnemy
  (return (Variables|Default|GetCounter%20Enemy)))

(fn GetDistancefromCounterEnemy
  (return (> (Transformation|GetDistanceTo (Components|GetOwner) (CallFunction|GetCounterEnemy)) (Variables|Default|GetTeleportDistance))))

(fn GetHUD
  (return (Variables|Default|GetHUD%20Ref)))

(fn SetHUD
  (params (HUDRef :type BP%20Hud%20Main%20Object%20Reference))
  (Variables|Default|SetHUD%20Ref HUDRef))

(fn SetFinisher
  (params (Finisher :type Boolean))
  (bind _hud_ref (Variables|Default|GetHUD%20Ref))
  (bind _ui_player_hud_ref (Variables|/Game/NoahsFolder/HUD/BP_Hud_Main.BP_Hud_Main_C|GetUI%20Player%20HUD%20Ref _hud_ref))
  (bind _output_get (Variables|Default|SetFinisher Finisher))
  (if _output_get
    (Default|SetCounterColour _ui_player_hud_ref "(R=0.973958,G=0.934521,B=0.070562,A=1.000000)")
    (else
      (Default|SetCounterColour _ui_player_hud_ref "(R=0.973958,G=0.973958,B=0.973958,A=1.000000)"))))

(fn GetFinisher
  (return (Variables|Default|GetFinisher)))

(fn GetFinisherAnims
  (return (Variables|Default|GetFinisherAnims)))

(fn GetAttackAnims
  (return (Variables|Default|GetAttackAnims)))

(fn GetDistancefromCurrentEnemy
  (return (> (Transformation|GetDistanceTo (Components|GetOwner) (CallFunction|GetCurrentEnemy)) (Variables|Default|GetTeleportDistance))))